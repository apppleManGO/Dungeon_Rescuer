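; BP_Game_npc is a talkable wizard NPC that plays an animation at BeginPlay and a cheer on interaction.
; Interact sends default or quest-cleared dialogue to BP_PlayerController based on the GameInstance's main-quest flag, then immediately calls EndDialogue on the instigating character.
; OnDialogueFinished clears the talking state, CanInteract always returns false, and failed casts print debug strings.
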(event `self.ReceiveBeginPlay`
  (`SkeletalMeshComponent.PlayAnimation` (`self.SkeletalMesh`) (`self.Montage`) false))

(event `CharaverCheer`
  (`SkeletalMeshComponent.PlayAnimation` (`self.SkeletalMesh`) (`self.MontageCheer`) false))

(event `self.Interact`
  (params (CharacterInstigator :type "US_Character Object Reference"))
  (bind _npc_master (`self.NPC_master`))
  (`self.CharaverCheer`)
  (bind _asbp_character (cast `/Game/BP/BP_Character` CharacterInstigator)
    (:`then`
      (bind _asbp_player_controller (cast `/Game/BP/BP_PlayerController` (`Pawn.GetController` _asbp_character))
        (:`then`
          (set `self.bIsTalking` true)
          (bind _asus_game_instance (cast `US_GameInstance` (`GameplayStatics.GetGameInstance`))
            (:`then`
              (if (`US_GameInstance.bIsMainQuestCleared` _asus_game_instance)
                (`/Game/BP/BP_PlayerController.dialogueEvent` _asbp_player_controller (`self.ClearDialogueLines`) _npc_master)
                (else
                  (`/Game/BP/BP_PlayerController.dialogueEvent` _asbp_player_controller (`self.DialogueLines`) _npc_master)))
              (bind _asbp_character_2 (cast `/Game/BP/BP_Character` CharacterInstigator))
              (`US_Character.EndDialogue` _asbp_character_2))
            (:`CastFailed`
              (`KismetSystemLibrary.PrintString` "설마 여기서 터졌나?"))))
        (:`CastFailed`
          (`KismetSystemLibrary.PrintString` "마법사 여기서도 터짐"))))
    (:`CastFailed`
      (`KismetSystemLibrary.PrintString` "마법사 여기서 터짐"))))

(fn `CanInteract`
  (params (CharacterInstigator :type "US_Character Object Reference"))
  (returns (ReturnValue :type Boolean))
  (return false))

(fn `OnDialogueFinished`
  (set `self.bDialogueFinished` true)
  (set `self.bIsTalking` false))

(fn `UserConstructionScript`)