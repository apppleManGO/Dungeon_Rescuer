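; BP_WoodenDoor is an interactable wooden door that toggles open and closed on Interact.
; On the authority, Interact flips DoorOpen and plays either the opening or closing timeline, yawing the mesh and reporting an AI noise event on each update.
; OnRep_DoorOpen plays the open or close sound at the door's location.
; CanInteract always returns false.
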(event `self.Interact`
  (params (CharacterInstigator :type "US_Character Object Reference"))
  (bind _staticmesh (`self.StaticMesh`))
  (`/Engine/EditorBlueprintResources/ActorMacros.Switch Has Authority`
    (:`Authority`
      (if (`self.DoorOpen`)
        (set `self.DoorOpen` false)
        (bind (_direction _rotationz) (`Timeline|Timeline`)
          (:`Update`
            (`SceneComponent.K2_SetRelativeRotation` _staticmesh (`KismetMathLibrary.MakeRotator` 0.0 0.0 _rotationz) false false)))
        (else
          (set `self.DoorOpen` true)
          (bind (_direction_2 _rotationz_2) (`Timeline|DoorOpening`)
            (:`Update`
              (`SceneComponent.K2_SetRelativeRotation` _staticmesh (`KismetMathLibrary.MakeRotator` 0.0 0.0 _rotationz_2) false false)))))
      (`AISense_Hearing.ReportNoiseEvent` (`self.K2_GetActorLocation`) 1.0 null))))

(fn `CanInteract`
  (params (CharacterInstigator :type "US_Character Object Reference"))
  (returns (ReturnValue :type Boolean))
  (return false))

(fn `OnRep_DoorOpen`
  (if (`self.DoorOpen`)
    (`GameplayStatics.PlaySoundAtLocation` "/Game/sound/npc/Drs_Chest_Large_Open_01.Drs_Chest_Large_Open_01" (`self.K2_GetActorLocation`) (struct) 1.0 1.0 0.0 null null null null)
    (else
      (`GameplayStatics.PlaySoundAtLocation` "/Game/sound/npc/Creaking_Door_Close_2.Creaking_Door_Close_2" (`self.K2_GetActorLocation`) (struct) 1.0 1.0 0.0 null null null null))))

(fn `UserConstructionScript`)