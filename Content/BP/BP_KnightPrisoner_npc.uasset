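; Rescuable knight prisoner NPC that plays a montage on BeginPlay.
; Interact grants XP to the instigator's player state, plays a cheer animation and increments the game state's rescued-NPC count.
; It then fires the player controller's dialogue event, calls EndDialogue on the character, activates Niagara after a delay and later destroys itself.
; CanInteract always returns false, although Interact is fully implemented.
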(event `self.ReceiveBeginPlay`
  (`SkeletalMeshComponent.PlayAnimation` (`self.SkeletalMesh`) (`self.Montage`) false))

(event `CharaverCheer`
  (`SkeletalMeshComponent.PlayAnimation` (`self.SkeletalMesh`) (`self.MontageCheer`) false))

(event `self.Interact`
  (params (CharacterInstigator :type "US_Character Object Reference"))
  (bind _asus_player_state (cast `US_PlayerState` (`Pawn.PlayerState` CharacterInstigator)))
  (`US_PlayerState.AddXp` _asus_player_state (`self.EarnedXp`))
  (`self.CharaverCheer`)
  (bind _asbp_game_state (cast `/Game/BP/BP_GameState` (`GameplayStatics.GetGameState`)))
  (`US_GameState.AddRescuedNPC` _asbp_game_state)
  (bind _asbp_character (cast `/Game/BP/BP_Character` CharacterInstigator))
  (bind _asbp_player_controller (cast `/Game/BP/BP_PlayerController` (`Pawn.GetController` _asbp_character)))
  (`/Game/BP/BP_PlayerController.dialogueEvent` _asbp_player_controller (`self.Dialoge`) (`self.NPC_knight`))
  (bind _asbp_character_2 (cast `/Game/BP/BP_Character` CharacterInstigator))
  (`US_Character.EndDialogue` _asbp_character_2)
  (`KismetSystemLibrary.Delay` 1.5)
  (`ActorComponent.SetActive` (`self.Niagara`) true true)
  (`KismetSystemLibrary.Delay` 3.0)
  (`self.K2_DestroyActor`))

(fn `CanInteract`
  (params (CharacterInstigator :type "US_Character Object Reference"))
  (returns (ReturnValue :type Boolean))
  (return false))

(fn `UserConstructionScript`)