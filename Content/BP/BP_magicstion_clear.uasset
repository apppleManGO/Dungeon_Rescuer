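; BP_magicstion_clear is an interactable NPC that appears only after the main quest is cleared.
; BeginPlay hides it and disables collision, then restores both if the game instance's IsMainQuestCleared flag is set.
; Interact plays a non-looping cheer animation, sends the clear dialogue to the player controller's DialogueEvent, then immediately calls EndDialogue on the instigating BP_Character.
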(event `self.ReceiveBeginPlay`
  (`parent.ReceiveBeginPlay`)
  (`self.SetActorHiddenInGame` true)
  (`self.SetActorEnableCollision` false)
  (bind _asus_game_instance (cast `US_GameInstance` (`GameplayStatics.GetGameInstance`)))
  (if (`US_GameInstance.bIsMainQuestCleared` _asus_game_instance)
    (`self.SetActorHiddenInGame` false)
    (`self.SetActorEnableCollision` true)))

(event `CustomEvent`
  (`SkeletalMeshComponent.PlayAnimation` (`self.SkeletalMesh`) (`self.MontageCheer`) false))

(event `self.Interact`
  (params (CharacterInstigator :type "US_Character Object Reference"))
  (`self.CustomEvent`)
  (bind _asbp_character (cast `/Game/BP/BP_Character` CharacterInstigator))
  (bind _asbp_player_controller (cast `/Game/BP/BP_PlayerController` (`Pawn.GetController` _asbp_character)))
  (`/Game/BP/BP_PlayerController.dialogueEvent` _asbp_player_controller (`self.Dialoge_clear`) (`self.NPC_knight_clear`))
  (bind _asbp_character_2 (cast `/Game/BP/BP_Character` CharacterInstigator))
  (`US_Character.EndDialogue` _asbp_character_2))

(fn `UserConstructionScript`
  (`parent.UserConstructionScript`))