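; BP_Potal is a portal trigger that gathers player characters before moving the session to the interior map.
; On authority, box overlaps add or remove characters in PlayerList, comparing each call's return value, not the list length, with the GameState's TotalPlayers.
; A match on either event reaches a shared DoOnce that flags the main quest cleared, fades in a widget and ServerTravels to Map_02_Interior after a delay.
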(event `self.ReceiveActorBeginOverlap`
  (params (OtherActor :type "Actor Object Reference")))

(event `self.Box.OnComponentBeginOverlap`
  (params (OverlappedComponent :type "PrimitiveComponent Object Reference") (OtherActor :type "Actor Object Reference") (OtherComp :type "PrimitiveComponent Object Reference") (OtherBodyIndex :type Integer) (bFromSweep :type Boolean) (SweepResult :type "HitResult Structure (by ref)"))
  (bind _asbp_character (cast `/Game/BP/BP_Character` OtherActor))
  (`/Engine/EditorBlueprintResources/ActorMacros.Switch Has Authority`
    (:`Authority`
      (bind _returnvalue (`KismetArrayLibrary.Array_AddUnique` (`self.PlayerList`) _asbp_character))
      (bind _asus_game_state (cast `US_GameState` (`GameplayStatics.GetGameState`))
        (:`then`
          (if (== _returnvalue (`US_GameState.TotalPlayers` _asus_game_state))
            (`/Engine/EditorBlueprintResources/StandardMacros.DoOnce` false :!label _label
              (:`Completed`
                (bind _asus_game_instance (cast `US_GameInstance` (`GameplayStatics.GetGameInstance`)))
                (set `US_GameInstance.bIsMainQuestCleared` true _asus_game_instance)
                (bind _returnvalue_2 (`|CreateWidget` "/Game/BP/WBP_Fade.WBP_Fade_C"))
                (`UserWidget.AddToViewport` _returnvalue_2 0)
                (`/Game/BP/WBP_Fade.FadeIn` _returnvalue_2)
                (`KismetSystemLibrary.Delay` 1.0)
                (`KismetSystemLibrary.ExecuteConsoleCommand` "ServerTravel Map_02_Interior?listen" null)))
            (else
              (`KismetSystemLibrary.PrintText` "not same count player"))))
        (:`CastFailed`
          (`KismetSystemLibrary.PrintString` "false gamestate" :!label _label_2))))))

(event `self.Box.OnComponentEndOverlap`
  (params (OverlappedComponent :type "PrimitiveComponent Object Reference") (OtherActor :type "Actor Object Reference") (OtherComp :type "PrimitiveComponent Object Reference") (OtherBodyIndex :type Integer))
  (bind _asbp_character (cast `/Game/BP/BP_Character` OtherActor))
  (`/Engine/EditorBlueprintResources/ActorMacros.Switch Has Authority`
    (:`Authority`
      (bind _returnvalue (`KismetArrayLibrary.Array_RemoveItem` (`self.PlayerList`) _asbp_character))
      (bind _asus_game_state (cast `US_GameState` (`GameplayStatics.GetGameState`))
        (:`then`
          (if (== _returnvalue (`US_GameState.TotalPlayers` _asus_game_state))
            (goto _label)
            (else
              (`KismetSystemLibrary.PrintText` "not smae player --"))))
        (:`CastFailed`
          (goto _label_2))))))

(fn `UserConstructionScript`)