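; Caged prisoner NPC that the party rescues by interacting while the game state holds the prison key.
; With the key, a timeline swings the door open and a one-time sequence runs dialogue, awards XP, cheers and records the rescue.
; Niagara effects play, then the prisoner is hidden and a portal spawns.
; Without the key it shows locked dialogue; an IsPrisonOpen RepNotify plays door sounds, and CanInteract always returns false.
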(event `self.ReceiveBeginPlay`
  (`SkeletalMeshComponent.PlayAnimation` (`self.SkeletalMesh`) (`self.Montage`) false))

(event `CharaverCheer`
  (`SkeletalMeshComponent.PlayAnimation` (`self.SkeletalMesh`) (`self.MontageCheer`) false))

(event `self.Interact`
  (params (CharacterInstigator :type "US_Character Object Reference"))
  (bind _skeletalmesh (`self.SkeletalMesh`))
  (bind _asbp_game_state (cast `/Game/BP/BP_GameState` (`GameplayStatics.GetGameState`))
    (:`then`
      (if (`US_GameState.bPartyHasPrisonKey` _asbp_game_state)
        (set `self.bIsPrisonOpen` true)
        (bind (_direction _rotationz) (`Timeline|Timeline`)
          (:`Update`
            (`SceneComponent.K2_SetRelativeRotation` (`self.Prision`) (`KismetMathLibrary.MakeRotator` 0.0 0.0 _rotationz) false false)
            (`/Engine/EditorBlueprintResources/StandardMacros.DoOnce` false
              (:`Completed`
                (bind _asus_player_state (cast `US_PlayerState` (`Pawn.PlayerState` CharacterInstigator))
                  (:`then`
                    (bind _asbp_character (cast `/Game/BP/BP_Character` CharacterInstigator))
                    (bind _asbp_player_controller (cast `/Game/BP/BP_PlayerController` (`Pawn.GetController` _asbp_character)))
                    (`/Game/BP/BP_PlayerController.dialogueEvent` _asbp_player_controller (`self.HaveKeyDialoge`) (`self.NPC_Magicion`))
                    (`US_Character.EndDialogue` _asbp_character)
                    (`US_PlayerState.AddXp` _asus_player_state (`self.EarnedXp`))
                    (`self.CharaverCheer`)
                    (bind _asbp_game_state_2 (cast `/Game/BP/BP_GameState` (`GameplayStatics.GetGameState`))
                      (:`then`
                        (`US_GameState.AddRescuedNPC` _asbp_game_state_2)
                        (`ActorComponent.SetActive` (`self.Niagara`) true true)
                        (`KismetSystemLibrary.Delay` 3.0)
                        (`SceneComponent.SetVisibility` _skeletalmesh false false)
                        (`PrimitiveComponent.SetCollisionEnabled` _skeletalmesh "NoCollision")
                        (`|SpawnActorFromClass` "/Game/BP/BP_Potal.BP_Potal_C" (`KismetMathLibrary.Conv_VectorToTransform` (`SceneComponent.K2_GetComponentLocation` (`self.SkeletalMesh`))) "AlwaysSpawn" "MultiplyWithRoot" null null))
                      (:`CastFailed`
                        (`KismetSystemLibrary.PrintString` "cast false gamestate"))))
                  (:`CastFailed`
                    (`KismetSystemLibrary.PrintString` "cast false platerstate")))))))
        (else
          (bind _asbp_character_2 (cast `/Game/BP/BP_Character` CharacterInstigator))
          (bind _asbp_player_controller_2 (cast `/Game/BP/BP_PlayerController` (`Pawn.GetController` _asbp_character_2)))
          (`/Game/BP/BP_PlayerController.dialogueEvent` _asbp_player_controller_2 (`self.noKeyDialoge`) (`self.NPC_Magicion`))
          (`US_Character.EndDialogue` _asbp_character_2))))
    (:`CastFailed`
      (`KismetSystemLibrary.PrintString` "not cast gamestate"))))

(fn `CanInteract`
  (params (CharacterInstigator :type "US_Character Object Reference"))
  (returns (ReturnValue :type Boolean))
  (return false))

(fn `OnRep_bIsPrisonOpen`
  (bind _returnvalue (`self.K2_GetActorLocation`))
  (if (`self.bIsPrisonOpen`)
    (`GameplayStatics.PlaySoundAtLocation` "/Game/sound/npc/Drs_Chest_Large_Open_01.Drs_Chest_Large_Open_01" _returnvalue (struct) 1.0 1.0 0.0 null null null null)
    (else
      (`GameplayStatics.PlaySoundAtLocation` "/Game/sound/npc/Door_Close_1.Door_Close_1" _returnvalue (struct) 1.0 1.0 0.0 null null null null))))

(fn `UserConstructionScript`)